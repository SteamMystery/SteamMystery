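; Bullet actor that leaves impact effects where it hits and removes itself after five seconds if nothing is struck.
; Tick repositions the Box component without sweep, multiplying its world location by the scaled forward vector rather than adding an offset, with no delta-time scaling.
; A Box hit spawns the NS_Impact Niagara system and a short-lived bullet-hole decal aligned to the surface normal, then destroys the actor.
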(event OnComponentHit(Box)
  (params (HitComponent :type Primitive%20Component%20Object%20Reference) (OtherActor :type Actor%20Object%20Reference) (OtherComp :type Primitive%20Component%20Object%20Reference) (NormalImpulse :type Vector :default "0, 0, 0") (Hit :type Hit%20Result%20Structure%20%28by%20ref%29))
  (Niagara|SpawnSystematLocation "/Game/VFX/NiagaraSystems/NS_Impact.NS_Impact" (.location Hit) (Math|Rotator|MakeRotfromZ (.normal Hit)))
  (Rendering|Decal|SpawnDecalatLocation "/Game/VFX/Materials/M_BulletHole.M_BulletHole" "7.000000,7.000000,7.000000" (.location Hit) (Math|Rotator|MakeRotfromX (.normal Hit)) 4.0)
  (Actor|DestroyActor))

(event Custom|BulletDestroy
  (Actor|DestroyActor))

(event EventBeginPlay
  (Utilities|Time|SetTimerbyEvent (delegate Custom|BulletDestroy) 5.0))

(event Collision|EventActorBeginOverlap
  (params (OtherActor :type Actor%20Object%20Reference)))

(event EventTick
  (params (DeltaSeconds :type Float%20%28single-precision%29))
  (bind _box (Variables|Default|GetBox))
  (Transformation|SetWorldLocation (Variables|Default|GetBox) (* (Transformation|GetWorldLocation _box) (* (Math|Vector|GetForwardVector _box) "100.000000,100.000000,100.000000")) false false))

(fn ConstructionScript)