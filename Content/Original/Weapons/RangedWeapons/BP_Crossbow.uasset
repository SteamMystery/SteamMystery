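; Crossbow ranged weapon Blueprint that syncs its skeletal mesh animation to firing and recharging by extending the parent weapon's functions.
; A successful Use plays the animation, and a successful StartRecharge jumps into it partway through.
; PlayAnimation scales the play rate so the remaining clip fits the Recharge stat's duration.
; Recharge runs the parent logic, then rewinds the mesh to the start, firing notifies.
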(fn ConstructionScript)

(fn Use
  (bind _returnvalue (|CallParentFunction))
  (if _returnvalue
    (Audio|Components|Audio|Play (Variables|Default|GetSkeletalMesh) false)
    (return _returnvalue)))

(fn PlayAnimation
  (params (InPos :type Float%20%28single-precision%29))
  (bind _skeletalmesh (Variables|Default|GetSkeletalMesh))
  (Components|Timeline|SetPlayRate _skeletalmesh (/ (- 5.666667 InPos) (.Value (Utilities|Map|Find (Class|Device|GetStats) "Recharge"))))
  (Components|Animation|SetPosition _skeletalmesh InPos true)
  (Audio|Components|Audio|Play _skeletalmesh false))

(fn StartRecharge
  (bind _returnvalue (|CallParentFunction))
  (if _returnvalue
    (CallFunction|PlayAnimation 3.0)
    (return _returnvalue)))

(fn Recharge
  (|CallParentFunction)
  (Components|Animation|SetPosition (Variables|Default|GetSkeletalMesh) 0.0 true))