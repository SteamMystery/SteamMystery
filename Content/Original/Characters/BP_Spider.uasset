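; BP_Spider is a spider character that adds a Steam attack on top of the attacks inherited from its parent class.
; On BeginPlay it caches the BP_Steam child actor, switches its spawning off and sets it to ignore the spider.
; The Attack override routes the Steam skill to SteamAttack, which raises the spawn rate for a half-second burst.
; Other skill names fall through to the parent Attack.
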(event Custom|SteamAttack
  (Default|SetSpawnRate (Variables|Default|GetAs%20BP%20Steam) 1.5e+03)
  (Utilities|FlowControl|Delay 0.5)
  (Default|SetSpawnRate (Variables|Default|GetAs%20BP%20Steam) 0.0))

(event EventBeginPlay
  (bind _asbp_steam (Utilities|Casting|CastToBP_Steam (Variables|/Script/Engine.ChildActorComponent|GetChildActor (Variables|Default|GetBP_Steam))))
  (bind _output_get (Variables|Default|SetAs%20BP%20Steam _asbp_steam))
  (Default|SetSpawnRate _output_get 0.0)
  (Variables|/Game/Original/Steam/BP_Steam.BP_Steam_C|SetIgnoredActors (Variables|Default|GetAs%20BP%20Steam) (Utilities|Array|MakeArray self)))

(fn ConstructionScript)

(fn Attack
  (params (SkillName :type Name :default "None"))
  (switch name SkillName
    (:Default
      (bind _returnvalue (|CallParentFunction SkillName))
      (return _returnvalue))
    (:Steam
      (CallFunction|SteamAttack)
      (return true))))