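; BP_MainMenuController is the player controller for the main menu, putting the menu widget on screen with UI-only input and a visible cursor.
; On BeginPlay it creates W_MainMenu, and on Destroyed it hides the cursor and restores game-only input.
; ShowOptions and HideOptions swap the main menu widget with the Options widget held in ALLUMG, reusing both instances rather than recreating them.
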(event Custom|Show%20Options
  (Widget|RemovefromParent (Variables|Default|GetWidget))
  (UserInterface|Viewport|AddtoViewport (Variables|/Game/UI/ALL_UMG.ALL_UMG_C|GetOptions (Variables|Default|GetALL_UMG)) 0))

(event Custom|Hide%20Options
  (Widget|RemovefromParent (Variables|/Game/UI/ALL_UMG.ALL_UMG_C|GetOptions (Variables|Default|GetALL_UMG)))
  (UserInterface|Viewport|AddtoViewport (Variables|Default|GetWidget) 0))

(event EventBeginPlay
  (bind _returnvalue (UserInterface|CreateWidget "/Game/UI/MainMenu/W_MainMenu.W_MainMenu_C"))
  (bind _output_get (Variables|Default|SetWidget _returnvalue))
  (UserInterface|Viewport|AddtoViewport _output_get 0)
  (Variables|Default|SetbShowMouseCursor true)
  (Input|SetInputModeUIOnly self _output_get "DoNotLock" false))

(event EventDestroyed
  (Variables|Default|SetbShowMouseCursor false)
  (Input|SetInputModeGameOnly self false))

(fn ConstructionScript)