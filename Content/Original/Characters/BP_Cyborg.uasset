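; BP_Cyborg is a character that adds Steam and Throw attacks, deferring other skill names to its parent's Attack.
; On BeginPlay it caches a child steam-wave actor, switches its emission off, sets it to ignore the Cyborg and registers itself with the melee trace component.
; Steam briefly pulses that actor's spawn rate after a short delay.
; Throw spawns a BP_Projectile from a spawn point toward the player's current location.
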(event Custom|SteamAttack
  (bind _as_bp_steam (Variables|Default|GetAs%20BP%20Steam))
  (Utilities|FlowControl|Delay 0.25)
  (Default|SetSpawnRate _as_bp_steam 7.5e+03)
  (Utilities|FlowControl|Delay 0.5)
  (Default|SetSpawnRate _as_bp_steam 0.0))

(event Custom|Throw%20Attack
  (bind _self self)
  (bind _projectile_spawn_point (Variables|Default|GetProjectile%20Spawn%20Point))
  (bind _returnvalue (Transformation|GetWorldLocation _projectile_spawn_point))
  (Game|SpawnActorfromClass "/Game/Original/Weapons/EnemyEquipment/BP_Projectile.BP_Projectile_C" (Math|Transform|MakeTransform _returnvalue "0, 0, 0" "1.000000,1.000000,1.000000") "Undefined" "MultiplyWithRoot" _self _returnvalue (Transformation|GetActorLocation (Game|Player|GetPlayerPawn 0)) 1.5e+03 _self))

(event EventBeginPlay
  (|CallParentFunction)
  (bind _asbp_steam_wave (Utilities|Casting|CastToBP_Steam_Wave (Variables|/Script/Engine.ChildActorComponent|GetChildActor (Variables|Default|GetBP_Steam))))
  (bind _output_get (Variables|Default|SetAs%20BP%20Steam _asbp_steam_wave))
  (Default|SetSpawnRate _output_get 0.0)
  (Variables|/Game/Original/Steam/BP_Steam_Wave.BP_Steam_Wave_C|SetIgnoredActors (Variables|Default|GetAs%20BP%20Steam) (Utilities|Array|MakeArray self))
  (Class|MeleeTraceComponent|SetWeapon (Variables|Default|GetMeleeTraceComponent) self)
  (Development|PrintString "Hello"))

(fn ConstructionScript)

(fn Attack
  (params (SkillName :type Name :default "None"))
  (switch name SkillName
    (:Default
      (bind _returnvalue (|CallParentFunction SkillName))
      (return _returnvalue))
    (:Steam
      (CallFunction|SteamAttack))
    (:Throw
      (CallFunction|ThrowAttack)))
  (return true))