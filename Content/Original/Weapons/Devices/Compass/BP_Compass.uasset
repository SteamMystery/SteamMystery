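; BP_Compass is a compass device that computes a heading toward the nearest actor tagged "Chest".
; Each Tick it scans those actors by 2D distance, updating MinDist and MinIndex, which the graph never resets between frames.
; It stores the relative look-at yaw to the selected chest in Angle, wrapping negatives into 0–360.
; With no chests, Angle gets a random value every frame.
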(event EventBeginPlay)

(event Collision|EventActorBeginOverlap
  (params (OtherActor :type Actor%20Object%20Reference)))

(event EventTick
  (params (DeltaSeconds :type Float%20%28single-precision%29))
  (bind _outactors (Actor|GetAllActorswithTag "Chest"))
  (if (> (Utilities|Array|Length _outactors) 0)
    (for (_array_element _array_index) _outactors
      (if (< (Math|Vector|Distance2D(Vector) (Transformation|GetActorLocation _array_element) (Transformation|GetActorLocation)) (Variables|Default|GetMinDist))
        (Variables|Default|SetMinDist (Math|Vector|Distance2D(Vector) (Transformation|GetActorLocation _array_element) (Transformation|GetActorLocation)))
        (Variables|Default|SetMinIndex _array_index)))
    (bind _result (Math|Float|NegateFloat (.yaw (Math|Rotator|FindRelativeLookatRotation (Transformation|GetActorTransform) (Transformation|GetActorLocation (Utilities|Array|Get(acopy) _outactors (Variables|Default|GetMinIndex))))))
      (:%20%20
        (if (< _result 0.0)
          (Variables|Default|SetAngle (+ 3.6e+02 (.yaw (Math|Rotator|FindRelativeLookatRotation (Transformation|GetActorTransform) (Transformation|GetActorLocation (Utilities|Array|Get(acopy) _outactors (Variables|Default|GetMinIndex)))))))
          (else
            (Variables|Default|SetAngle (.yaw (Math|Rotator|FindRelativeLookatRotation (Transformation|GetActorTransform) (Transformation|GetActorLocation (Utilities|Array|Get(acopy) _outactors (Variables|Default|GetMinIndex))))))))))
    (else
      (Variables|Default|SetAngle (Math|Random|RandomFloatinRange 0.0 3.6e+02)))))

(fn ConstructionScript)